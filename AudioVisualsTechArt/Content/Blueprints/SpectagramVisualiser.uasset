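; Audio spectrum visualiser actor that spawns a grid of VisualiserCube actors and stretches their height to the music.
; On BeginPlay it plays the AudioHost's sound on its own audio component and spawns the cubes, wrapping rows at MaxGrid.
; Each Tick it copies GlobalIntensity and ConstantBandStrength (Constant-Q bands) from the first AudioHost.
; Playback-percent events set each cube's Z scale from its band strength, global intensity and LocalScaling.
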(event `self.ReceiveTick`
  (params (DeltaSeconds :type "Float (single-precision)"))
  ;[1 1 1] Recieve Data from Audio Host
  (bind _outactors (`GameplayStatics.GetAllActorsOfClass` "/Game/Blueprints/AudioHost.AudioHost_C"))
  (bind _output (`|GetArrayItem` _outactors))
  (set `self.Global Intensity` (`/Game/Blueprints/AudioHost.GlobalIntensity` _output))
  (set `self.Constant Band Strength` (`/Game/Blueprints/AudioHost.ConstantBandStrength` _output)))

(event `self.ReceiveBeginPlay`
  (bind _outactors (`GameplayStatics.GetAllActorsOfClass` "/Game/Blueprints/AudioHost.AudioHost_C"))
  (`|ExecutionSequence`
    (:`then_0`
      ;[1 1 1] Set Audio Reference
      (bind _output_get (set `self.RefMusic` (`/Game/Blueprints/AudioHost.Sound` (`|GetArrayItem` _outactors))))
      (`AudioComponent.SetSound` (`self.Audio`) _output_get))
    (:`then_1`
      ;[1 1 1] Generate Cubes
      (bind _spawnedcubes (`self.CreateCubes` (`self.Cube Number`) (`self.Spacing`)))
      (set `self.Spawned Cubes` _spawnedcubes))
    (:`then_2`
      ;[1 1 1] Reference ConstantQ to Scale Cubes
      (add `AudioComponent.OnAudioPlaybackPercent` (`self.Audio`) (delegate `CustomEvent`))
      (`ActorComponent.Activate` (`self.Audio`) false))))

(event `CustomEvent`
  (params (PlayingSoundWave :type "SoundWave Object Reference") (PlaybackPercent :type "Float (single-precision)"))
  ;[1 1 1] Reference ConstantQ to Scale Cubes
  (`self.ConstantVisualiserScaling` (`self.Spawned Cubes`)))

(fn `ConstantVisualiserScaling`
  (params (`Visualiser Cubes` :type "Array of /Game/Objects/VisualiserCube Object Reference"))
  (for (_array_element _array_index) (`self.Constant Band Strength`)
    (`SceneComponent.SetWorldScale3D` (`/Game/Objects/VisualiserCube.Cube` (`|GetArrayItem` `Visualiser Cubes` _array_index)) (`KismetMathLibrary.MakeVector` 0.1 0.1 (* (* (`self.Global Intensity`) (`self.LocalScaling`)) _array_element)))))

(fn `CreateCubes`
  (params (CubeNumber :type Integer) (Spacing :type "Float (double-precision)"))
  (returns (SpawnedCubes :type "Array of /Game/Objects/VisualiserCube Object Reference"))
  (bind (_returnvalue_x _returnvalue_y _returnvalue_z) (`KismetMathLibrary.BreakVector` (`SceneComponent.K2_GetComponentLocation` (`self.DefaultSceneRoot`))))
  (for _index (range (+ CubeNumber 1))
    (bind (_remainder _returnvalue) (`KismetMathLibrary.FMod` (`KismetMathLibrary.Conv_IntToDouble` _index) (`self.MaxGrid`)))
    (`|SpawnActorFromClass` "/Game/Objects/VisualiserCube.VisualiserCube_C" (`KismetMathLibrary.MakeTransform` (`KismetMathLibrary.MakeVector` (+ _returnvalue_x (* _remainder Spacing)) (+ _returnvalue_y (* _returnvalue Spacing)) _returnvalue_z) (struct) (0.1 0.1 0.1)) "Undefined" "OverrideRootScale" null null))
  (bind _outactors (`GameplayStatics.GetAllActorsOfClass` "/Game/Objects/VisualiserCube.VisualiserCube_C"))
  (return _outactors))

(fn `UserConstructionScript`)